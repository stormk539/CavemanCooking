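; Pickup actor that the player collects with the Interact input, apparently a carrot drop.
; Overlapping its Box enables input on the actor for the first player and shows a PressE_WBP prompt; leaving disables input and removes the prompt.
; Pressing Interact calls AddCarrotMessage on the player character, removes the prompt and destroys the pickup.
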(event `self.Box.OnComponentBeginOverlap`
  (params (OverlappedComponent :type "PrimitiveComponent Object Reference") (OtherActor :type "Actor Object Reference") (OtherComp :type "PrimitiveComponent Object Reference") (OtherBodyIndex :type Integer) (bFromSweep :type Boolean) (SweepResult :type "HitResult Structure (by ref)"))
  (if (== OtherActor (`GameplayStatics.GetPlayerCharacter` 0))
    (`self.EnableInput` (`GameplayStatics.GetPlayerController` 0))
    (bind _returnvalue (`|CreateWidget` "/Game/Widgets/PressE_WBP.PressE_WBP_C"))
    (bind _output_get (set `self.WidgetRef` _returnvalue))
    (`UserWidget.AddToViewport` _output_get 0)))

(event `self.Box.OnComponentEndOverlap`
  (params (OverlappedComponent :type "PrimitiveComponent Object Reference") (OtherActor :type "Actor Object Reference") (OtherComp :type "PrimitiveComponent Object Reference") (OtherBodyIndex :type Integer))
  (bind _widgetref (`self.WidgetRef`))
  (if (== (`GameplayStatics.GetPlayerCharacter` 0) OtherActor)
    (`self.DisableInput` (`GameplayStatics.GetPlayerController` 0))
    (if (`Widget.bIsEnabled` _widgetref)
      (`Widget.RemoveFromParent` _widgetref))))

(event `InputAction|Interact`
  (params (Key :type "Key Structure"))
  (:`Pressed`
    (message `/Game/Blueprints/Interfaces/AddToCharacter_BPI.AddCarrot` (`GameplayStatics.GetPlayerCharacter` 0))
    (`Widget.RemoveFromParent` (`self.WidgetRef`))
    (`self.K2_DestroyActor`)))

(fn `UserConstructionScript`)