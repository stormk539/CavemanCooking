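; Berry bush Blueprint that the player harvests by holding Interact inside its Box, granting berries once through AddBerryMessage.
; Box overlap toggles input, the HoldInput_WBP widget and a gate on the press.
; A retriggerable delay of MaxHoldTime checks that Interact is still held, then recolors the Cube and disables interaction.
; Meanwhile, a timer's elapsed time feeds widget progress through a self-calling delayed update, resetting on release.
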(event `InputAction|Interact`
  (params (Key :type "Key Structure"))
  (:`Pressed`
    (set `self.IsHeld?` true)
    (`/Engine/EditorBlueprintResources/StandardMacros.Gate` true :!label _label
      (:`Exit`
        (`|ExecutionSequence`
          (:`then_0`
            (`KismetSystemLibrary.RetriggerableDelay` (`self.MaxHoldTime`))
            (if (`self.IsHeld?`)
              (`self.FinishEvents`)))
          (:`then_1`
            (`self.Timer`)
            (`self.Update Widget`))))))
  (:`Released`
    (set `self.IsHeld?` false)))

(event `self.Box.OnComponentBeginOverlap`
  (params (OverlappedComponent :type "PrimitiveComponent Object Reference") (OtherActor :type "Actor Object Reference") (OtherComp :type "PrimitiveComponent Object Reference") (OtherBodyIndex :type Integer) (bFromSweep :type Boolean) (SweepResult :type "HitResult Structure (by ref)"))
  (if (== OtherActor (`GameplayStatics.GetPlayerCharacter` 0))
    (if (`self.CanInteract`)
      (`self.EnableInput` (`GameplayStatics.GetPlayerController` 0))
      (bind _returnvalue (`|CreateWidget` "/Game/Widgets/HoldInput_WBP.HoldInput_WBP_C"))
      (bind _output_get (set `self.WidgetRef` _returnvalue))
      (`UserWidget.AddToViewport` _output_get 0)
      (set `/Game/Widgets/HoldInput_WBP.MaxHoldTime` (`self.MaxHoldTime`) _output_get)
      (goto _label :!via `Open`))))

(event `self.Box.OnComponentEndOverlap`
  (params (OverlappedComponent :type "PrimitiveComponent Object Reference") (OtherActor :type "Actor Object Reference") (OtherComp :type "PrimitiveComponent Object Reference") (OtherBodyIndex :type Integer))
  (if (== OtherActor (`GameplayStatics.GetPlayerCharacter` 0))
    (`self.DisableInput` (`GameplayStatics.GetPlayerController` 0))
    (if (`Widget.bIsEnabled` (`self.WidgetRef`))
      (`Widget.RemoveFromParent` (stale `self.Box.OnComponentBeginOverlap` _returnvalue))
      (goto _label :!via `Close`))))

(event `Stop Timer`
  (`KismetSystemLibrary.K2_PauseTimerHandle` (stale `Timer` _returnvalue)))

(event `Timer`
  (bind _returnvalue (`KismetSystemLibrary.K2_SetTimerDelegate` (delegate `Timer`) (`self.MaxHoldTime`))))

(event `Update Widget`
  (bind _widgetref (`self.WidgetRef`))
  (if (`self.IsHeld?`)
    (set `/Game/Widgets/HoldInput_WBP.HoldTime` (`KismetSystemLibrary.K2_GetTimerElapsedTimeHandle` (stale `Timer` _returnvalue)) _widgetref)
    (`KismetSystemLibrary.Delay` 0.1)
    (`self.Update Widget`)
    (else
      (`self.Stop Timer`)
      (set `/Game/Widgets/HoldInput_WBP.HoldTime` 0.0 _widgetref))))

(fn `FinishEvents`
  (`PrimitiveComponent.SetMaterial` (`self.Cube`) 0 "/Game/LevelPrototyping/Materials/MI_Solid_Blue.MI_Solid_Blue")
  (set `self.CanInteract` false)
  (`Widget.RemoveFromParent` (`self.WidgetRef`))
  (message `/Game/Blueprints/Interfaces/AddToCharacter_BPI.AddBerry` (`GameplayStatics.GetPlayerCharacter` 0) (`self.BerriesDropped`)))

(fn `UserConstructionScript`)