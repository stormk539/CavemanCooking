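; Customer spawn point that creates an NPC at its own location on BeginPlay and sends it to a free chair.
; FindChair claims the first unoccupied Chair_BP and passes it to the NPC's MoveNPC along with a reference to this spawner.
; A running count of claimed chairs sets Full once it equals the chair total, blocking further SpawnCustomer calls.
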(event `self.ReceiveBeginPlay`
  (`self.SpawnCustomer`))

(event `self.SpawnCustomer`
  ;[1 1 1] Spawn Customer
  (if (not (`self.Full?`))
    (bind _returnvalue (`|SpawnActorFromClass` "/Game/AI/TestNPC/NPC.NPC_C" (`KismetMathLibrary.MakeTransform` (`self.K2_GetActorLocation`)) "Undefined" "OverrideRootScale" null null))
    (set `self.Customer` _returnvalue)
    (`self.FindChair`)))

(event `FindChair`
  ;[1 1 1] Find Chair
  (bind _outactors (`GameplayStatics.GetAllActorsOfClass` "/Game/Blueprints/Chairs/Chair_BP.Chair_BP_C"))
  (for _array_element _outactors
    (if (not (`/Game/Blueprints/Chairs/Chair_BP.HasCustomer?` _array_element))
      (`/Engine/EditorBlueprintResources/StandardMacros.IncrementInt` (`self.Passes`)
        (:`  `
          (set `/Game/Blueprints/Chairs/Chair_BP.HasCustomer?` true _array_element)
          (`self.MoveNPC` (`self.Customer`) _array_element self)
          (break)))))
  (if (== (`KismetArrayLibrary.Array_Length` _outactors) (`self.Passes`))
    (set `self.Full?` true)))

(fn `UserConstructionScript`)