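; SaladStation01 is a cooking station actor that lets the player open a salad station screen when standing nearby.
; Entering its box trigger enables the actor's input and shows a Press E prompt widget; leaving disables input and removes all such prompts.
; Pressing Interact removes the prompt, creates the SaladStation_WBP widget, and switches to UI-only input with the mouse cursor shown.
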(event `InputAction|Interact`
  (params (Key :type "Key Structure"))
  (bind _returnvalue (`GameplayStatics.GetPlayerController` 0))
  (:`Pressed`
    (`Widget.RemoveFromParent` (`self.WidgetRef`))
    (bind _returnvalue_2 (`|CreateWidget` "/Game/Widgets/SaladStation_WBP.SaladStation_WBP_C"))
    (`UserWidget.AddToViewport` _returnvalue_2 0)
    (`WidgetBlueprintLibrary.SetInputMode_UIOnlyEx` _returnvalue null)
    (set `PlayerController.bShowMouseCursor` true _returnvalue)))

(event `self.Box.OnComponentBeginOverlap`
  (params (OverlappedComponent :type "PrimitiveComponent Object Reference") (OtherActor :type "Actor Object Reference") (OtherComp :type "PrimitiveComponent Object Reference") (OtherBodyIndex :type Integer) (bFromSweep :type Boolean) (SweepResult :type "HitResult Structure (by ref)"))
  (if (== OtherActor (`GameplayStatics.GetPlayerCharacter` 0))
    (`self.EnableInput` (`GameplayStatics.GetPlayerController` 0))
    (bind _returnvalue (`|CreateWidget` "/Game/Widgets/PressE_WBP.PressE_WBP_C"))
    (bind _output_get (set `self.WidgetRef` _returnvalue))
    (`UserWidget.AddToViewport` _output_get 0)))

(event `self.Box.OnComponentEndOverlap`
  (params (OverlappedComponent :type "PrimitiveComponent Object Reference") (OtherActor :type "Actor Object Reference") (OtherComp :type "PrimitiveComponent Object Reference") (OtherBodyIndex :type Integer))
  (if (== (`GameplayStatics.GetPlayerCharacter` 0) OtherActor)
    (`self.DisableInput` (`GameplayStatics.GetPlayerController` 0))
    (bind _foundwidgets (`WidgetBlueprintLibrary.GetAllWidgetsOfClass` "/Game/Widgets/PressE_WBP.PressE_WBP_C"))
    (for _array_element _foundwidgets
      (`Widget.RemoveFromParent` _array_element))))

(fn `UserConstructionScript`)