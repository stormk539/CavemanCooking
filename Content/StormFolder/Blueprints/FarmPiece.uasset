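; FarmPiece is a farm plot actor that grows carrots from the player's seeds and lets the player harvest them.
; Overlapping TriggerBox while idle calls GrowingCarrot, then harvests any finished carrot into the character's Carrots count.
; Growing spends a seed, shows the mesh, then chains three timelines as timed stages, nudging it upward after each.
; IsGrowing blocks re-triggering, staying set if no seed is available, and the mesh height is never reset.
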(event `self.TriggerBox.OnComponentBeginOverlap`
  (params (OverlappedComponent :type "PrimitiveComponent Object Reference") (OtherActor :type "Actor Object Reference") (OtherComp :type "PrimitiveComponent Object Reference") (OtherBodyIndex :type Integer) (bFromSweep :type Boolean) (SweepResult :type "HitResult Structure (by ref)"))
  ;[1 1 1] Player Picks Up Grown Food
  (if (not (`self.IsGrowing?`))
    (`self.GrowingCarrot`)
    (bind _asbp_third_person_character (cast `/Game/ThirdPerson/Blueprints/BP_ThirdPersonCharacter` OtherActor))
    (if (`self.SeedDone?`)
      (`SceneComponent.SetVisibility` (`self.Carrot`) false false)
      (bind _result (`/Engine/EditorBlueprintResources/StandardMacros.IncrementInt` (`/Game/ThirdPerson/Blueprints/BP_ThirdPersonCharacter.Carrots` _asbp_third_person_character))
        (:`  `
          (`KismetSystemLibrary.PrintString` (`KismetStringLibrary.Conv_IntToString` _result))
          (`KismetSystemLibrary.PrintString` "You got a carrot!")
          (set `self.SeedDone?` false))))))

(event `GrowingCarrot`
  (bind _carrot (`self.Carrot`))
  ;[1 1 1] Grow Carrot
  (set `self.IsGrowing?` true)
  (bind _asbp_third_person_character (cast `/Game/ThirdPerson/Blueprints/BP_ThirdPersonCharacter` (`GameplayStatics.GetPlayerCharacter` 0)))
  (bind _carrotseed (`/Game/ThirdPerson/Blueprints/BP_ThirdPersonCharacter.CarrotSeed` _asbp_third_person_character))
  (if (> _carrotseed 0)
    (`/Engine/EditorBlueprintResources/StandardMacros.DecrementInt` _carrotseed
      (:`  `
        (`SceneComponent.SetVisibility` (`self.Carrot`) true false)
        (`KismetSystemLibrary.Delay` 3.0)
        (`Timeline|Timeline_2`
          (:`Finished`
            (`SceneComponent.K2_SetWorldLocation` _carrot (+ (`SceneComponent.K2_GetComponentLocation` _carrot) (0.0 0.0 5.0)) false false)
            (`Timeline|Timeline_3`
              (:`Finished`
                (`SceneComponent.K2_SetWorldLocation` _carrot (+ (`SceneComponent.K2_GetComponentLocation` _carrot) (0.0 0.0 5.0)) false false)
                (`Timeline|Timeline_4`
                  (:`Finished`
                    (`SceneComponent.K2_SetWorldLocation` _carrot (+ (`SceneComponent.K2_GetComponentLocation` _carrot) (0.0 0.0 5.0)) false false)
                    (set `self.SeedDone?` true)
                    (set `self.IsGrowing?` false)))))))))))

(fn `UserConstructionScript`)