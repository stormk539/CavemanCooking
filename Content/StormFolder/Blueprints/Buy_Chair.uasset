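; Buy_Chair is a purchasable chair actor that the player buys with the third-person character's Currency.
; Overlapping its Box enables input and shows a BuyChair widget; leaving removes the widget and disables input.
; Pressing Interact with enough currency makes the chair appear by setting material and collision on its parts, then deducts the cost and prints the balance.
; Nothing records the purchase or filters which actor overlaps.
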(event `InputAction|Interact`
  (params (Key :type "Key Structure"))
  ;[1 1 1] Hiding/Making Chair Appear
  (:`Pressed`
    (`self.BuyChair`)))

(event `BuyChair`
  (bind _seat (`self.Seat`))
  ;[1 1 1] Hiding/Making Chair Appear
  (bind _asbp_third_person_character (cast `/Game/ThirdPerson/Blueprints/BP_ThirdPersonCharacter` (`GameplayStatics.GetPlayerCharacter` 0)))
  (bind _currency (`/Game/ThirdPerson/Blueprints/BP_ThirdPersonCharacter.Currency` _asbp_third_person_character))
  (if (>= _currency 100)
    (`PrimitiveComponent.SetMaterial` _seat 0 "/Game/StormFolder/Materials/Chair_Color.Chair_Color")
    (`PrimitiveComponent.SetMaterial` (`self.Back`) 0 "/Game/StormFolder/Materials/Chair_Color.Chair_Color")
    (`PrimitiveComponent.SetMaterial` (`self.Leg1`) 0 "/Game/StormFolder/Materials/Chair_Color.Chair_Color")
    (`PrimitiveComponent.SetMaterial` (`self.Leg2`) 0 "/Game/StormFolder/Materials/Chair_Color.Chair_Color")
    (`PrimitiveComponent.SetMaterial` (`self.Leg3`) 0 "/Game/StormFolder/Materials/Chair_Color.Chair_Color")
    (`PrimitiveComponent.SetMaterial` (`self.Leg4`) 0 "/Game/StormFolder/Materials/Chair_Color.Chair_Color")
    (`PrimitiveComponent.SetCollisionEnabled` _seat "QueryAndPhysics")
    (`PrimitiveComponent.SetCollisionEnabled` (`self.Back`) "QueryAndPhysics")
    (`PrimitiveComponent.SetCollisionEnabled` (`self.Leg1`) "QueryAndPhysics")
    (`PrimitiveComponent.SetCollisionEnabled` (`self.Leg2`) "QueryAndPhysics")
    (`PrimitiveComponent.SetCollisionEnabled` (`self.Leg3`) "QueryAndPhysics")
    (`PrimitiveComponent.SetCollisionEnabled` (`self.Leg4`) "QueryAndPhysics")
    (bind _output_get (set `/Game/ThirdPerson/Blueprints/BP_ThirdPersonCharacter.Currency` (- _currency 100) _asbp_third_person_character))
    (`KismetSystemLibrary.PrintString` (`KismetStringLibrary.Conv_IntToString` _output_get))))

(event `self.Box.OnComponentBeginOverlap`
  (params (OverlappedComponent :type "PrimitiveComponent Object Reference") (OtherActor :type "Actor Object Reference") (OtherComp :type "PrimitiveComponent Object Reference") (OtherBodyIndex :type Integer) (bFromSweep :type Boolean) (SweepResult :type "HitResult Structure (by ref)"))
  ;[1 1 1] Creating Widget/Allowing Player Interaction
  (`self.EnableInput` (`GameplayStatics.GetPlayerController` 0))
  (bind _returnvalue (`|CreateWidget` "/Game/StormFolder/Widgets/BuyChair.BuyChair_C"))
  (`UserWidget.AddToViewport` _returnvalue 0))

(event `self.Box.OnComponentEndOverlap`
  (params (OverlappedComponent :type "PrimitiveComponent Object Reference") (OtherActor :type "Actor Object Reference") (OtherComp :type "PrimitiveComponent Object Reference") (OtherBodyIndex :type Integer))
  ;[1 1 1] Creating Widget/Allowing Player Interaction
  (bind _foundwidgets (`WidgetBlueprintLibrary.GetAllWidgetsOfClass` "/Game/StormFolder/Widgets/BuyChair.BuyChair_C"))
  (`Widget.RemoveFromParent` _foundwidgets)
  (`self.DisableInput` (`GameplayStatics.GetPlayerController` 0)))

(fn `UserConstructionScript`)